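; BP_Button_Letterbox is an interactable button that plays an animated letterbox effect.
; Its Interact event plays a timeline from the start, which writes the "Letterbox Height" scalar into the MPC_Postprocess material parameter collection on every update.
; A playing flag ignores further interactions until the timeline finishes.
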(event `/Game/Exam/BI_Interact.Interact`
  (if (not (`self.Is Letterboxd Playing?`))
    (set `self.Is Letterboxd Playing?` true)
    (bind (_direction _letterbox_height) (`Timeline|Timeline_0` :!via `PlayFromStart`)
      (:`Update`
        (`KismetMaterialLibrary.SetScalarParameterValue` "/Game/Materials/MPC_Postprocess.MPC_Postprocess" "Letterbox Height" _letterbox_height))
      (:`Finished`
        (set `self.Is Letterboxd Playing?` false)))))

(fn `UserConstructionScript`
  (`parent.UserConstructionScript`))
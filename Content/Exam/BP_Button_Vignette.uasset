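; BP_Button_Vignette is an interactable button that plays a screen vignette effect when its Interact event fires.
; Interact starts a timeline that drives the Vignette Size and Vignette Offset X scalar parameters in the MPC_Postprocess material parameter collection.
; An IsVignettePlaying flag blocks retriggering until the timeline finishes.
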(event `/Game/Exam/BI_Interact.Interact`
  (if (not (`self.Is Vignette Playing?`))
    (set `self.Is Vignette Playing?` true)
    (bind (_direction _vignette_size _vignette_offset_x) (`Timeline|Timeline_0` :!via `PlayFromStart`)
      (:`Update`
        (`KismetMaterialLibrary.SetScalarParameterValue` "/Game/Materials/MPC_Postprocess.MPC_Postprocess" "Vignette Size" _vignette_size)
        (`KismetMaterialLibrary.SetScalarParameterValue` "/Game/Materials/MPC_Postprocess.MPC_Postprocess" "Vignette Offset X" _vignette_offset_x))
      (:`Finished`
        (set `self.Is Vignette Playing?` false)))))

(fn `UserConstructionScript`
  (`parent.UserConstructionScript`))
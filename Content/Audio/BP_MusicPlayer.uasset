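; Music player Blueprint that plays the track held in CurrentAudio through its AudioComponent.
; BeginPlay calls StartMusic, which assigns the sound and fades it in.
; ChangeMusic fades out, waits for the fade to finish, then assigns CurrentAudio again and fades back in.
; One FadeDuration drives both fades and the delay, and nothing in these graphs sets CurrentAudio.
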(event `self.ReceiveBeginPlay`
  (`self.Start Music`))

(event `Event ChangeMusic`
  (bind _audiocomponent (`self.AudioComponent`))
  (bind _fadeduration (`self.FadeDuration`))
  (`AudioComponent.FadeOut` _audiocomponent _fadeduration 0.0 "Linear")
  (`KismetSystemLibrary.Delay` _fadeduration)
  (`AudioComponent.SetSound` _audiocomponent (`self.CurrentAudio`))
  (`AudioComponent.FadeIn` _audiocomponent (`self.FadeDuration`) 1.0 0.0 "Linear"))

(fn `Start Music`
  (bind _audiocomponent (`self.AudioComponent`))
  (`AudioComponent.SetSound` _audiocomponent (`self.CurrentAudio`))
  (`AudioComponent.FadeIn` _audiocomponent (`self.FadeDuration`) 1.0 0.0 "Linear"))

(fn `UserConstructionScript`)
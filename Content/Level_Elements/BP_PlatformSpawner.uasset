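; Level element actor that repeatedly spawns platforms of the Platform class at its own transform.
; On BeginPlay it spawns the first platform and multiplies that platform's TimeGap by GapMultiplier to set its own spawn interval.
; Tick feeds a Delay of that interval, which acts as a repeating timer for further spawns through the shared SpawnPlatform function.
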(event `self.ReceiveBeginPlay`
  (bind _spawnedplatform (`self.SpawnPlatform`))
  (set `self.TimeGap` (* (`/Game/Level_Elements/Platform/BP_Platform.TimeGap` _spawnedplatform) (`self.GapMultiplier`))))

(event `self.ReceiveTick`
  (params (DeltaSeconds :type "Float (single-precision)"))
  (`KismetSystemLibrary.Delay` (`self.TimeGap`))
  (`self.SpawnPlatform`))

(fn `SpawnPlatform`
  (returns (SpawnedPlatform :type "/Game/Level_Elements/Platform/BP_Platform Object Reference"))
  (bind _returnvalue (`|SpawnActorFromClass` (`self.Platform`) (`self.GetTransform`) "Undefined" "OverrideRootScale" null null))
  (return _returnvalue))

(fn `UserConstructionScript`)
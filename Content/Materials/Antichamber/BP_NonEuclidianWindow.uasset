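; Antichamber-style non-Euclidean window Blueprint that applies position-aware materials to an object and its surrounding walls.
; On BeginPlay it creates dynamic instances of the object material and the Antichamber frame material.
; Both receive the world locations of the PointA and PointB components as vector parameters and are assigned to the Object and AntichamberWalls meshes.
; The construction script is empty.
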(event `self.ReceiveBeginPlay`
  (bind _returnvalue (`KismetMathLibrary.Conv_VectorToLinearColor` (`SceneComponent.K2_GetComponentLocation` (`self.Point A`))))
  (bind _returnvalue_2 (`KismetMathLibrary.Conv_VectorToLinearColor` (`SceneComponent.K2_GetComponentLocation` (`self.Point B`))))
  (`|ExecutionSequence`
    (:`then_0`
      ;[1 1 1] Object
      (bind _returnvalue_3 (`KismetMaterialLibrary.CreateDynamicMaterialInstance` (`self.ObjectMaterial`)))
      (`MaterialInstanceDynamic.SetVectorParameterValue` _returnvalue_3 "Point A" _returnvalue)
      (`MaterialInstanceDynamic.SetVectorParameterValue` _returnvalue_3 "Point B" _returnvalue_2)
      (`PrimitiveComponent.SetMaterial` (`self.Object`) 0 _returnvalue_3))
    (:`then_1`
      ;[1 1 1] Walls
      (bind _returnvalue_4 (`KismetMaterialLibrary.CreateDynamicMaterialInstance` "/Game/Materials/Antichamber/M_05_Antichamber_Frame.M_05_Antichamber_Frame"))
      (`MaterialInstanceDynamic.SetVectorParameterValue` _returnvalue_4 "Point A" _returnvalue)
      (`MaterialInstanceDynamic.SetVectorParameterValue` _returnvalue_4 "Point B" _returnvalue_2)
      (`PrimitiveComponent.SetMaterial` (`self.AntichamberWalls`) 0 _returnvalue_4))))

(fn `UserConstructionScript`)